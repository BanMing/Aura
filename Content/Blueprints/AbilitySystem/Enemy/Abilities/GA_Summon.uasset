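; Enemy summon ability that spawns random minions at generated locations around a shaman.
; It turns the avatar toward its combat target and plays the summon montage, waiting for a gameplay event before placing ground Niagara effects at shuffled spawn points.
; After a short delay, a staggered loop spawns AI-controlled minions facing the target.
; The avatar's minion count rises per spawn and falls when each minion is destroyed.
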(event `self.K2_ActivateAbility`
  (bind _returnvalue (`self.GetAvatarActorFromActorInfo`))
  (bind _returnvalue_2 (+ (`|GetArrayItem` (`self.Spawn Locations`) (`self.Spawn Location Index`)) (0.0 0.0 70.0)))
  (set `self.Spawn Location Index` 0)
  (bind _returnvalue_3 (message `EnemyInterface.GetCombatTarget` _returnvalue))
  (message `CombatInterface.SetFacingTarget` _returnvalue (`Actor.K2_GetActorLocation` _returnvalue_3))
  (`AbilityTask_PlayMontageAndWait.CreatePlayMontageAndWaitProxy` "None" "/Game/Assets/Enemies/Shaman/Animations/AM_Shaman_Summon.AM_Shaman_Summon"
    (:`then`
      (`AbilityTask_WaitGameplayEvent.WaitGameplayEvent` (struct :`TagName` "Montage.Attack.1") null true
        (:`EventReceived`
          (bind _returnvalue_4 (`self.GetSpawnLocations`))
          (set `self.Spawn Locations` _returnvalue_4)
          (`KismetArrayLibrary.Array_Shuffle` (`self.Spawn Locations`))
          (for _array_element (`self.Spawn Locations`)
            (`NiagaraFunctionLibrary.SpawnSystemAtLocation` "/Game/Assets/Effects/Combat/NS_GroundSummon.NS_GroundSummon" _array_element))
          ;[1 1 1] Spawn Minion
          (`KismetSystemLibrary.Delay` 0.75)
          (if (< (`self.Spawn Location Index`) (`KismetArrayLibrary.Array_Length` (`self.Spawn Locations`))) :!label _label
            (bind _returnvalue_5 (message `EnemyInterface.GetCombatTarget` (`self.GetAvatarActorFromActorInfo`)))
            (bind _returnvalue_6 (`|SpawnActorFromClass` (`self.GetRandomMinionClass`) (`KismetMathLibrary.MakeTransform` _returnvalue_2 (`KismetMathLibrary.Conv_VectorToRotator` (- (`Actor.K2_GetActorLocation` _returnvalue_5) _returnvalue_2))) "AlwaysSpawn" "MultiplyWithRoot" null null))
            (add `Actor.OnDestroyed` _returnvalue_6 (delegate `OnDestroyed`))
            (`Pawn.SpawnDefaultController` _returnvalue_6)
            (message `CombatInterface.IncrementMinionCount` (`self.GetAvatarActorFromActorInfo`) 1)
            (`/Engine/EditorBlueprintResources/StandardMacros.IncrementInt` (`self.Spawn Location Index`)
              (:`  `
                (`KismetSystemLibrary.Delay` 0.2)
                (goto _label)))
            (else
              (`self.K2_EndAbility`))))))
    (:`OnInterrupted`
      (`self.K2_EndAbility` :!label _label_2))
    (:`OnCancelled`
      (goto _label_2))))

(event `OnDestroyed`
  (params (DestroyedActor :type "Actor Object Reference"))
  ;[1 1 1] Spawn Minion
  (message `CombatInterface.IncrementMinionCount` (`self.GetAvatarActorFromActorInfo`) -1))