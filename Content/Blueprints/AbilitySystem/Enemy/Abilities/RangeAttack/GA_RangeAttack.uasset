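; Enemy ranged attack gameplay ability that fires a projectile at the avatar's current combat target.
; On activation it turns the avatar toward the target and plays a random tagged montage.
; The montage's gameplay event triggers the projectile spawn from its tagged combat socket, with an optional pitch override.
; The ability ends right after spawning, leaving the montage to play out.
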(event `self.K2_ActivateAbility`
  (bind _returnvalue (`self.GetAvatarActorFromActorInfo`))
  (bind _returnvalue_2 (message `EnemyInterface.GetCombatTarget` _returnvalue))
  (bind _returnvalue_3 (`Actor.K2_GetActorLocation` _returnvalue_2))
  (message `CombatInterface.SetFacingTarget` _returnvalue _returnvalue_3)
  (bind _output_get (set `self.TaggedMontage` (`self.GetRandomTaggedMontage`)))
  (bind (_montage _montagetag _combatsockettag) (break `TaggedMontage` _output_get))
  (`AbilityTask_PlayMontageAndWait.CreatePlayMontageAndWaitProxy` "None" _montage 1.0 "None" false
    (:`then`
      (`AbilityTask_WaitGameplayEvent.WaitGameplayEvent` _montagetag null true
        (:`EventReceived`
          (`self.SpawnProjectileByTag` _returnvalue_3 _combatsockettag (`self.Override Pitch`) 25.0)
          (`self.K2_EndAbility`))))))