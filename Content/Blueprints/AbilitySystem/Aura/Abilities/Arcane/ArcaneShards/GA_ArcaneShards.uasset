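; Arcane Shards gameplay ability that shows a magic circle and, on input press, casts a burst of damaging shards at the targeted ground point.
; A montage event spawns BP_PointCollection, which supplies ground points at a random yaw, then hides the circle.
; A looping timer steps through the points, applying damage to live players in radius except the caster and executing a shard GameplayCue at each.
; The ability ends shortly after the last point.
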(event `self.K2_ActivateAbility`
  (`|ExecutionSequence`
    (:`then_0`
      (message `PlayerInterface.ShowMagicCircle` (`self.GetAvatarActorFromActorInfo`) null))
    (:`then_1`
      (`AbilityTask_WaitInputPress.WaitInputPress` false
        (:`OnPress`
          (bind (_asynctaskproxy _datahandle) (`AbilityTask_TargetDataUnderMouse.CreateTargetDataUnderMouse`)
            (:`ValidDataEvent`
              (bind (_returnvalue_bblockinghit _returnvalue_binitialoverlap _returnvalue_time _returnvalue_distance _returnvalue_location _returnvalue_impactpoint) (`GameplayStatics.BreakHitResult` (`AbilitySystemBlueprintLibrary.GetHitResultFromTargetData` _datahandle)))
              (set `self.PointCollectionLocation` _returnvalue_impactpoint)
              (message `CombatInterface.SetFacingTarget` (`self.GetAvatarActorFromActorInfo`) (`self.PointCollectionLocation`))
              (`AbilityTask_PlayMontageAndWait.CreatePlayMontageAndWaitProxy` "None" "/Game/Assets/Characters/Aura/Animations/Abilities/AM_Cast_ArcaneShards_Short.AM_Cast_ArcaneShards_Short" 1.0 "None" false
                (:`then`
                  (`AbilityTask_WaitGameplayEvent.WaitGameplayEvent` (struct :`TagName` "Event.Montage.ArcaneShards") null true
                    (:`EventReceived`
                      (bind _returnvalue (`|SpawnActorFromClass` "/Game/Blueprints/AbilitySystem/Aura/Abilities/Arcane/ArcaneShards/BP_PointCollection.BP_PointCollection_C" (`KismetMathLibrary.MakeTransform` (`self.PointCollectionLocation`)) "Undefined" "MultiplyWithRoot" null null))
                      (bind _output_get (set `self.PointCollection` _returnvalue))
                      (set `self.Ground Points` (`PointCollection.GetGroundPoints` _output_get (`self.PointCollectionLocation`) (`self.Num Points`) (`KismetMathLibrary.RandomFloatInRange` 0.0 360.0)))
                      (bind _returnvalue_2 (`KismetSystemLibrary.K2_SetTimerDelegate` (delegate `SpawnShard`) (`self.ShardSpawnDeltaTime`) true))
                      (set `self.ShardSpawnTimer` _returnvalue_2)
                      (`self.SpawnShard`)
                      (message `PlayerInterface.HideMagicCircle` (`self.GetAvatarActorFromActorInfo`)))))))))))))

(event `SpawnShard`
  (bind _returnvalue (`self.GetAvatarActorFromActorInfo`))
  (if (< (`self.Count`) (`self.Num Points`))
    (set `self.ShardsSpawnLocation` (`SceneComponent.K2_GetComponentLocation` (`|GetArrayItem` (`self.Ground Points`) (`self.Count`))))
    (bind _outoverlappingactors (`AuraAbilitySystemLibrary.GetLivePlayersWithinRadius` _returnvalue (`|MakeArray` _returnvalue) (`self.RadialDamageOuterRadius`) (`self.ShardsSpawnLocation`)))
    (bind _output_get (set `self.PlayerToDamage` _outoverlappingactors))
    (for _array_element _output_get
      (`AuraAbilitySystemLibrary.ApplyDamageEffect` (`self.MakeDamageEffectParamsFromClassDefaults` _array_element (`self.ShardsSpawnLocation`))))
    (`/Engine/EditorBlueprintResources/StandardMacros.IncrementInt` (`self.Count`)
      (:`  `
        (`self.K2_ExecuteGameplayCueWithParams` (struct :`TagName` "GameplayCue.ArcaneShards") (`AbilitySystemBlueprintLibrary.MakeGameplayCueParameters` 0.0 0.0 (struct) (struct) (struct) (struct) (struct) (`self.ShardsSpawnLocation`)))))
    (else
      (`KismetSystemLibrary.K2_ClearAndInvalidateTimerHandle` (`self.ShardSpawnTimer`))
      (`KismetSystemLibrary.Delay` 0.2)
      (`self.K2_EndAbility`))))