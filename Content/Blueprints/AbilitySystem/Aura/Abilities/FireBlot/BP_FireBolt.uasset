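; BP_FireBolt is the Fire Bolt projectile actor, which explodes when it stops moving.
; Each Tick, MakeGokaboomIfNoMove stores the current location and compares the squared distance from the previous frame's location to MinDistancePerFrame.
; At or below that threshold, it plays the impact sound, spawns the Niagara explosion at the projectile's location and destroys the actor.
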(event `self.ReceiveBeginPlay`)

(event `self.ReceiveTick`
  (params (DeltaSeconds :type "Float (single-precision)"))
  (`self.MakeGokaboomIfNoMove`))

(fn `MakeGokaboomIfNoMove`
  (set `self.LastFrameLocation` (`self.ProjectileLocation`))
  (set `self.ProjectileLocation` (`self.K2_GetActorLocation`))
  (if (<= (`KismetMathLibrary.VSizeSquared` (- (`self.ProjectileLocation`) (`self.LastFrameLocation`))) (`self.Min Distance Per Frame`))
    (`GameplayStatics.SpawnSoundAtLocation` "/Game/Assets/Sounds/Abilities/FireBolt/sfx_FireBolt_Impact.sfx_FireBolt_Impact" (`self.ProjectileLocation`) (struct) 1.0 1.0 0.0 null null)
    (`NiagaraFunctionLibrary.SpawnSystemAtLocation` "/Game/Assets/Effects/Projectiles/FireExplosion/NS_FireExplosion2.NS_FireExplosion2" (`self.ProjectileLocation`))
    (`self.K2_DestroyActor`)))

(fn `UserConstructionScript`)