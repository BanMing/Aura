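; Fireball actor for the FireBlast ability that flies out along its forward vector, then returns to ReturnToActor and explodes.
; On the authority, two chained timelines lerp its location out to the apex, then back toward that actor's live position.
; Within ExplodeDistance it calls OnHit, applies radial damage params with upward-angled knockback to nearby live players, excluding its owner, then destroys itself.
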(event `self.ReceiveBeginPlay`)

(event `self.StartOutgoingTimeline`
  (`/Engine/EditorBlueprintResources/ActorMacros.Switch Has Authority`
    (:`Authority`
      ;[1 1 1] Store Initial Location and Apex Location
      (set `self.InitialLocation` (`self.K2_GetActorLocation`))
      (set `self.ApexLocation` (+ (`self.InitialLocation`) (* (`self.GetActorForwardVector`) (`self.TravelDistance`))))
      (bind (_direction _outgoingtrack) (`Timeline|OutgoingTimeline`)
        (:`Update`
          (`self.K2_SetActorLocation` (`KismetMathLibrary.VLerp` (`self.InitialLocation`) (`self.ApexLocation`) _outgoingtrack)))
        (:`Finished`
          (bind (_direction_2 _returningtrack) (`Timeline|ReturningTimeline`)
            (:`Update`
              (`self.K2_SetActorLocation` (`KismetMathLibrary.VLerp` (`self.ApexLocation`) (`self.K2_GetActorLocation` (`self.ReturnToActor`)) _returningtrack))
              (if (`self.IsWithinExplodeDistance`)
                (`self.OnHit`)
                (`self.ApplyExplosionDamageEffect`)
                (`self.K2_DestroyActor`)))))))))

(fn `ApplyExplosionDamageEffect`
  (`AuraAbilitySystemLibrary.SetRadialDamageEffectParam` (`self.ExplosionDamageParams`) true 50.0 300.0 (`self.K2_GetActorLocation`))
  (bind _outoverlappingactors (`AuraAbilitySystemLibrary.GetLivePlayersWithinRadius` self (`|MakeArray` (`self.GetOwner`) self :!type "Actor Object Reference") 300.0 (`self.K2_GetActorLocation`)))
  (for _array_element _outoverlappingactors
    (`AuraAbilitySystemLibrary.SetTargetASCEffectParam` (`self.ExplosionDamageParams`) _array_element)
    (bind _returnvalue (- (`self.K2_GetActorLocation` _array_element) (`self.K2_GetActorLocation`)))
    (`AuraAbilitySystemLibrary.SetDeathImpulseDirectionEffectParam` (`self.ExplosionDamageParams`) _returnvalue)
    (bind (_returnvalue_roll _returnvalue_pitch _returnvalue_yaw) (`KismetMathLibrary.BreakRotator` (`KismetMathLibrary.MakeRotFromX` _returnvalue)))
    (`AuraAbilitySystemLibrary.SetKnockbackDirectionEffectParam` (`self.ExplosionDamageParams`) (`KismetMathLibrary.GetForwardVector` (`KismetMathLibrary.MakeRotator` _returnvalue_roll 45.0 _returnvalue_yaw)) 800.0)
    (`AuraAbilitySystemLibrary.ApplyDamageEffect` (`self.ExplosionDamageParams`))))

(fn `IsWithinExplodeDistance`
  (returns (ReturnValue :type Boolean))
  (return (<= (`KismetMathLibrary.VSize` (- (`self.K2_GetActorLocation`) (`self.K2_GetActorLocation` (`self.ReturnToActor`)))) (`self.ExplodeDistance`))))

(fn `UserConstructionScript`)