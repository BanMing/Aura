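; Melee attack gameplay ability that turns the avatar toward its combat target and plays a random montage from its tagged attack montages.
; The montage's gameplay event triggers a radius check at the combat socket matching that tag, damaging live players found there, excluding the attacker.
; A debug sphere shows the hit area, and the ability ends only after that event, as montage completion or interruption is not handled.
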(event `self.K2_ActivateAbility`
  (bind _returnvalue (`self.GetAvatarActorFromActorInfo`))
  (bind _returnvalue_2 (`self.GetAvatarActorFromActorInfo`))
  (bind _returnvalue_3 (message `EnemyInterface.GetCombatTarget` _returnvalue))
  (message `CombatInterface.SetFacingTarget` _returnvalue (`Actor.K2_GetActorLocation` _returnvalue_3))
  (bind _returnvalue_4 (message `CombatInterface.GetAttackMontages` _returnvalue))
  (bind _output_get (set `self.TaggedMontage` (`|GetArrayItem` _returnvalue_4 (`KismetMathLibrary.RandomIntegerInRange` 0 (- (`KismetArrayLibrary.Array_Length` _returnvalue_4) 1)))))
  (bind (_montage _montagetag) (break `TaggedMontage` _output_get))
  (`AbilityTask_PlayMontageAndWait.CreatePlayMontageAndWaitProxy` "None" _montage
    (:`then`
      (`AbilityTask_WaitGameplayEvent.WaitGameplayEvent` _montagetag null
        (:`EventReceived`
          (bind _returnvalue_5 (message `CombatInterface.GetCombatSocketLocation` _returnvalue_2 _montagetag))
          (`KismetSystemLibrary.DrawDebugSphere` _returnvalue_5 45.0 12 (struct :`R` 0.88 :`A` 1.0) 5.0)
          (bind _outoverlappingactors (`AuraAbilitySystemLibrary.GetLivePlayersWithinRadius` _returnvalue_2 (`|MakeArray` _returnvalue_2) 45.0 _returnvalue_5))
          (for _array_element _outoverlappingactors
            (`self.CauseDamage` _array_element))
          (`self.K2_EndAbility`))))))