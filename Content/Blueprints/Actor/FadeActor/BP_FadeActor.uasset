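; BP_FadeActor is an actor whose static mesh fades through a timeline, played by FadeOut and reversed by Fadein.
; Construction caches the original materials and applies dynamic instances built from separate fade materials.
; Timeline updates reapply those instances and drive their "Fade" parameter.
; At finish, a value of 1 restores the original materials, and an optional flag switches Visibility collision to Block at 1 or Ignore at 0.
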(event `/Game/Blueprints/Actor/FadeActor/BP_FadeInterface.Fade Out`
  (bind (_direction _fade) (`Timeline|Fading` :!label _label)
    (:`Update`
      (for (_array_element _array_index) (`self.DynamicMaterialInstance`)
        (`PrimitiveComponent.SetMaterial` (`self.StaticMesh`) _array_index _array_element)
        (`MaterialInstanceDynamic.SetScalarParameterValue` _array_element "Fade" _fade)))
    (:`Finished`
      (`self.Fade Finished` _fade))))

(event `/Game/Blueprints/Actor/FadeActor/BP_FadeInterface.Fade In`
  (goto _label :!via `Reverse`))

(fn `Fade Finished`
  (params (Fade :type "Float (double-precision)"))
  (bind _staticmesh (`self.StaticMesh`))
  (if (>= Fade 1.0)
    (`self.Set Original Materials`)
    (if (`self.BlockVisibity`)
      (`PrimitiveComponent.SetCollisionResponseToChannel` _staticmesh "ECC_Visibility" "ECR_Block"))
    (elif (<= Fade 0.0)
      (if (`self.BlockVisibity`)
        (`PrimitiveComponent.SetCollisionResponseToChannel` _staticmesh "ECC_Visibility" "ECR_Ignore")))))

(fn `Set Materials to Dynamic Instance`
  (for (_array_element _array_index) (`self.DynamicMaterialInstance`)
    (`PrimitiveComponent.SetMaterial` (`self.StaticMesh`) _array_index _array_element)))

(fn `Set Original Materials`
  (for (_array_element _array_index) (`self.OriginalMaterials`)
    (`PrimitiveComponent.SetMaterial` (`self.StaticMesh`) _array_index _array_element)))

(fn `UserConstructionScript`
  (`KismetArrayLibrary.Array_Clear` (`self.DynamicMaterialInstance`))
  (set `self.OriginalMaterials` (`MeshComponent.GetMaterials` (`self.StaticMesh`)))
  (for _array_element (`self.FadeMaterialsInstance`)
    (bind _returnvalue (`KismetMaterialLibrary.CreateDynamicMaterialInstance` _array_element))
    (`KismetArrayLibrary.Array_Add` (`self.DynamicMaterialInstance`) _returnvalue))
  (`self.Set Materials to Dynamic Instance`))