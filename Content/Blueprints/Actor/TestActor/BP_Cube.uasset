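; BP_Cube is a test actor that displays orientation debug text on screen every tick.
; It prints its rotation, the X vector derived from that rotation, and its forward vector in separately colored lines, each prefixed with a Name variable.
; Consecutive message keys offset from PrintKey make each line update in place.
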(event `self.ReceiveTick`
  (params (DeltaSeconds :type "Float (single-precision)"))
  (`KismetSystemLibrary.PrintString` (`KismetStringLibrary.BuildString_Rotator` (`self.Name`) "    " (`self.K2_GetActorRotation`)) true true (struct :`G` 0.66 :`B` 1.0 :`A` 1.0) 2.0 (`KismetStringLibrary.Conv_StringToName` (`KismetStringLibrary.Conv_IntToString` (`self.PrintKey`))))
  (`KismetSystemLibrary.PrintString` (`KismetStringLibrary.BuildString_Vector` (`self.Name`) "   " (`KismetMathLibrary.Conv_RotatorToVector` (`self.K2_GetActorRotation`))) true true (struct :`R` 0.57 :`A` 1.0) 2.0 (`KismetStringLibrary.Conv_StringToName` (`KismetStringLibrary.Conv_IntToString` (+ (`self.PrintKey`) 1))))
  (`KismetSystemLibrary.PrintString` (`KismetStringLibrary.BuildString_Vector` (`self.Name`) "   " (`self.GetActorForwardVector`)) true true (struct :`R` 0.06 :`G` 1.0 :`B` 0.88411 :`A` 1.0) 2.0 (`KismetStringLibrary.Conv_StringToName` (`KismetStringLibrary.Conv_IntToString` (+ (`self.PrintKey`) 2)))))

(fn `UserConstructionScript`)