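; Base enemy character Blueprint that handles spawn, death-style dissolve and health bar visuals.
; Timelines scale the mesh on BeginPlay and drive a "Dissolve" scalar on dynamic materials, with a separate timeline for the weapon.
; SetFacingTarget feeds a location to Motion Warping as "FacingTarget".
; Health and max-health handlers both write raw values to the widget's front bar percent, but their delegate bindings here never run.
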(event `self.ReceiveBeginPlay`
  (bind (_direction _scaletrack) (`Timeline|SpawnTimeline`)
    (:`Update`
      (`SceneComponent.SetRelativeScale3D` (`self.Mesh`) (`KismetMathLibrary.MakeVector` _scaletrack _scaletrack _scaletrack)))))

(event `OnHealthChanged_Event` :!signature `self.OnHealthChanged`
  (params (NewValue :type "Float (single-precision)"))
  ;[1 1 1] Health Changed
  (bind _aswbp_enemy_health_bar (cast `/Game/Blueprints/UI/ProgressBar/WBP_EnemyHealthBar` (`WidgetComponent.GetWidget` (`self.HealthBar`))))
  (`ProgressBar.SetPercent` (`/Game/Blueprints/UI/ProgressBar/WBP_ProgressBar.ProgressBar_Front` _aswbp_enemy_health_bar) NewValue))

(event `OnMaxHealthChanged_Event` :!signature `self.OnMaxHealthChanged`
  (params (NewValue :type "Float (single-precision)"))
  ;[1 1 1] Health Changed
  (bind _aswbp_enemy_health_bar (cast `/Game/Blueprints/UI/ProgressBar/WBP_EnemyHealthBar` (`WidgetComponent.GetWidget` (`self.HealthBar`))))
  (`ProgressBar.SetPercent` (`/Game/Blueprints/UI/ProgressBar/WBP_ProgressBar.ProgressBar_Front` _aswbp_enemy_health_bar) NewValue))

(event `self.StartDissolveTimeline`
  (params (MaterialInstanceDynamic :type "MaterialInstanceDynamic Object Reference"))
  ;[1 1 1] Dissolve
  (bind (_direction _dissolvetrack) (`Timeline|DissolveTimeline`)
    (:`Update`
      (`MaterialInstanceDynamic.SetScalarParameterValue` MaterialInstanceDynamic "Dissolve" _dissolvetrack))))

(event `self.StartWeaponDissolveTimeline`
  (params (MaterialInstanceDynamic :type "MaterialInstanceDynamic Object Reference"))
  ;[1 1 1] Dissolve
  (bind (_direction _weapondissolvetrack) (`Timeline|WeaponDissolveTimeline`)
    (:`Update`
      (`MaterialInstanceDynamic.SetScalarParameterValue` MaterialInstanceDynamic "Dissolve" _weapondissolvetrack))))

(event `CombatInterface.SetFacingTarget`
  (params (TargetLocation :type "Vector Structure (by ref)"))
  ;[1 1 1] Facing Target
  (`MotionWarpingComponent.AddOrUpdateWarpTargetFromLocation` (`self.MotionWarping`) "FacingTarget" TargetLocation))

(fn `UserConstructionScript`)